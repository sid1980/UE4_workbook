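; BP_LampEditableHard1 is a lamp actor that toggles when E is pressed.
; Its construction script gives PointLightHard and the Cube's dynamic emissive material one random color.
; E checks light visibility: LampOn hides the light and raises Emissive, while LampOff shows it and zeroes Emissive.
; Both events share a DoOnce that creates and stores a runtime material instance, and their color writes target a parameter named None.
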(event `self.ReceiveBeginPlay`
  (`self.EnableInput` (`GameplayStatics.GetPlayerController` 0)))

(event `Key|E`
  (params (Key :type "Key Structure"))
  (:`Pressed`
    (if (`SceneComponent.IsVisible` (`self.PointLightHard`))
      (`self.LampOn`)
      (else
        (`self.LampOff`)))))

(event `LampOn`
  (`SceneComponent.SetVisibility` (`self.PointLightHard`) false false)
  (`|ExecutionSequence`
    (:`then_0`
      (`/Engine/EditorBlueprintResources/StandardMacros.DoOnce` false :!label _label
        (:`Completed`
          (bind _returnvalue (`PrimitiveComponent.CreateDynamicMaterialInstance` (`self.Cube`) 0 "/Game/M_Emissive_Inst.M_Emissive_Inst" "None"))
          (set `self.InstanceLink` _returnvalue))))
    (:`then_1`
      (`MaterialInstanceDynamic.SetScalarParameterValue` (`self.InstanceLink`) "Emissive" 5.0)
      (`MaterialInstanceDynamic.SetVectorParameterValue` (`self.InstanceLink`) "None" (struct :`R` 1.0 :`G` 0.901327 :`B` 0.068713 :`A` 1.0)))))

(event `LampOff`
  (`SceneComponent.SetVisibility` (`self.PointLightHard`) true false)
  (`|ExecutionSequence`
    (:`then_0`
      (goto _label))
    (:`then_1`
      (`MaterialInstanceDynamic.SetScalarParameterValue` (`self.InstanceLink`) "Emissive" 0.0)
      (`MaterialInstanceDynamic.SetVectorParameterValue` :`self` (`self.InstanceLink`)))))

(fn `UserConstructionScript`
  (`|ExecutionSequence`
    (:`then_0`
      (bind _output_get (set `self.color` (make `LinearColor` (`KismetMathLibrary.RandomFloatInRange` 0.0 1.0) (`KismetMathLibrary.RandomFloatInRange` 0.0 1.0) (`KismetMathLibrary.RandomFloatInRange` 0.0 1.0))))
      (`LightComponent.SetLightColor` (`self.PointLightHard`) _output_get true))
    (:`then_1`
      (bind _returnvalue (`PrimitiveComponent.CreateDynamicMaterialInstance` (`self.Cube`) 0 "/Game/M_Emissive_Inst.M_Emissive_Inst" "None"))
      (`MaterialInstanceDynamic.SetVectorParameterValue` _returnvalue "Color" (`self.color`)))))
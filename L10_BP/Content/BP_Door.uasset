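; BP_Door is a proximity door that rescales its SMWall component based on the player's distance.
; Each Tick it compares that distance to a fixed threshold and prints TRUE or FALSE as debug output.
; Two cross-resetting DoOnce nodes apply the scale only when the range state changes: smaller when the player is near, larger in Y and Z when away.
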(event `self.ReceiveTick`
  (params (DeltaSeconds :type "Float (single-precision)"))
  (bind _sm_wall (`self.SM_Wall`))
  (if (< (`self.GetDistanceTo` (`GameplayStatics.GetPlayerCharacter` 0)) 250.0)
    (`KismetSystemLibrary.PrintString` "TRUE" true false (struct :`G` 0.66 :`B` 1.0 :`A` 1.0) 0.0)
    (`|ExecutionSequence`
      (:`then_0`
        (`/Engine/EditorBlueprintResources/StandardMacros.DoOnce` false :!label _label
          (:`Completed`
            (`SceneComponent.SetWorldScale3D` _sm_wall (0.5 0.5 0.5)))))
      (:`then_1`
        (goto _label_2 :!via `Reset`)))
    (else
      (`KismetSystemLibrary.PrintString` "FALSE" true false (struct :`G` 0.66 :`B` 1.0 :`A` 1.0) 0.0)
      (`|ExecutionSequence`
        (:`then_0`
          (`/Engine/EditorBlueprintResources/StandardMacros.DoOnce` false :!label _label_2
            (:`Completed`
              (`SceneComponent.SetWorldScale3D` _sm_wall (0.5 0.75 0.75)))))
        (:`then_1`
          (goto _label :!via `Reset`))))))

(fn `UserConstructionScript`)
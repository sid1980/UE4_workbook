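; Interactable lamp with a configurable Color, which the construction script applies to its point light and a dynamic emissive material.
; Overlapping the Box shows a PressE prompt and enables input, so E toggles between LampOn and LampOff.
; These events share a DoOnce-created material instance for emissive changes and swap an optional referenced mesh's material.
; The naming runs opposite to the light: LampOn hides PointLightHard while raising emissive, and LampOff does the reverse.
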(event `self.Box.OnComponentBeginOverlap`
  (params (OverlappedComponent :type "PrimitiveComponent Object Reference") (OtherActor :type "Actor Object Reference") (OtherComp :type "PrimitiveComponent Object Reference") (OtherBodyIndex :type Integer) (bFromSweep :type Boolean) (SweepResult :type "HitResult Structure (by ref)"))
  (`self.EnableInput` (`GameplayStatics.GetPlayerController` 0))
  (`SceneComponent.SetVisibility` (`self.Press E`) true false))

(event `self.Box.OnComponentEndOverlap`
  (params (OverlappedComponent :type "PrimitiveComponent Object Reference") (OtherActor :type "Actor Object Reference") (OtherComp :type "PrimitiveComponent Object Reference") (OtherBodyIndex :type Integer))
  (`self.DisableInput` (`GameplayStatics.GetPlayerController` 0))
  (`SceneComponent.SetVisibility` (`self.Press E`) false false))

(event `self.ReceiveBeginPlay`
  (`SceneComponent.SetVisibility` (`self.Press E`) false false)
  (`self.DisableInput` (`GameplayStatics.GetPlayerController` 0))
  (bind _meshreference (`self.MeshReference`)
    (:`then`
      (`PrimitiveComponent.SetMaterial` (`StaticMeshActor.StaticMeshComponent` _meshreference) 0 "/Game/M_Emissive_Inst.M_Emissive_Inst"))
    (:`else`)))

(event `Key|E`
  (params (Key :type "Key Structure"))
  (:`Pressed`
    (if (`SceneComponent.IsVisible` (`self.PointLightHard`))
      (`self.LampOn`)
      (else
        (`self.LampOff`)))))

(event `LampOn`
  (`SceneComponent.SetVisibility` (`self.PointLightHard`) false false)
  (`|ExecutionSequence`
    (:`then_0`
      (`/Engine/EditorBlueprintResources/StandardMacros.DoOnce` false :!label _label
        (:`Completed`
          (bind _returnvalue (`PrimitiveComponent.CreateDynamicMaterialInstance` (`self.Cube`) 0 "/Game/M_Emissive_Inst.M_Emissive_Inst" "None"))
          (set `self.InstanceLink` _returnvalue))))
    (:`then_1`
      (`MaterialInstanceDynamic.SetScalarParameterValue` (`self.InstanceLink`) "Emissive" 5.0)
      (`MaterialInstanceDynamic.SetVectorParameterValue` (`self.InstanceLink`) "None" (struct :`R` 1.0 :`G` 0.901327 :`B` 0.068713 :`A` 1.0))
      (bind _meshreference (`self.MeshReference`)
        (:`then`
          (`PrimitiveComponent.SetMaterial` (`StaticMeshActor.StaticMeshComponent` _meshreference) 0 "/Game/M_White.M_White"))
        (:`else`)))))

(event `LampOff`
  (`SceneComponent.SetVisibility` (`self.PointLightHard`) true false)
  (`|ExecutionSequence`
    (:`then_0`
      (goto _label))
    (:`then_1`
      (`MaterialInstanceDynamic.SetScalarParameterValue` (`self.InstanceLink`) "Emissive" 0.0)
      (`MaterialInstanceDynamic.SetVectorParameterValue` :`self` (`self.InstanceLink`))
      (bind _meshreference (`self.MeshReference`)
        (:`then`
          (`PrimitiveComponent.SetMaterial` (`StaticMeshActor.StaticMeshComponent` _meshreference) 0 "/Game/M_Emissive_Inst.M_Emissive_Inst"))
        (:`else`)))))

(fn `UserConstructionScript`
  (`|ExecutionSequence`
    (:`then_0`
      (bind _output_get (set `self.color` (`self.color`)))
      (`LightComponent.SetLightColor` (`self.PointLightHard`) _output_get true))
    (:`then_1`
      (bind _returnvalue (`PrimitiveComponent.CreateDynamicMaterialInstance` (`self.Cube`) 0 "/Game/M_Emissive_Inst.M_Emissive_Inst" "None"))
      (`MaterialInstanceDynamic.SetVectorParameterValue` _returnvalue "Color" (`self.color`)))))
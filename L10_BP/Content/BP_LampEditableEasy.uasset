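; BP_LampEditableEasy is a lamp actor that toggles PointLightEasy when the player presses E, with input enabled for player 0 at BeginPlay.
; The key handler checks light visibility and calls LampOn or LampOff, which set visibility, swap the Cube's material and print debug text.
; The event names are inverted: LampOn hides the light and LampOff shows it.
; An unconnected dynamic-material emissive setup never runs.
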(event `self.ReceiveBeginPlay`
  (`self.EnableInput` (`GameplayStatics.GetPlayerController` 0)))

(event `Key|E`
  (params (Key :type "Key Structure"))
  (:`Pressed`
    (if (`SceneComponent.IsVisible` (`self.PointLightEasy`))
      (`self.LampOn`)
      (else
        (`self.LampOff`)))))

(event `LampOn`
  (`KismetSystemLibrary.PrintString` "EasyOn" true true (struct :`G` 0.66 :`B` 1.0 :`A` 1.0) 0.0)
  (`SceneComponent.SetVisibility` (`self.PointLightEasy`) false false)
  (`PrimitiveComponent.SetMaterial` (`self.Cube`) 0 "/Game/M_Emissive_Inst.M_Emissive_Inst"))

(event `LampOff`
  (`KismetSystemLibrary.PrintString` "EasyOff" true true (struct :`G` 0.66 :`B` 1.0 :`A` 1.0) 0.0)
  (`SceneComponent.SetVisibility` (`self.PointLightEasy`) true false)
  (`PrimitiveComponent.SetMaterial` (`self.Cube`) 0 "/Game/M_Emissive.M_Emissive"))

(fn `UserConstructionScript`)
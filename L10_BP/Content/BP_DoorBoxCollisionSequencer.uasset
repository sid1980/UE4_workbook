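; Swinging door Blueprint that opens when something overlaps its BoxFront trigger and closes when the overlap ends.
; The DoorAnim timeline plays from start or reverses from end, lerping SMWall's relative rotation.
; Each update compares wall and player world X to pick the swing direction, away from a 90-degree closed yaw.
; Level sequence, distance-based scaling and offset experiments remain as unconnected nodes.
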(event `self.BoxFront.OnComponentBeginOverlap`
  (params (OverlappedComponent :type "PrimitiveComponent Object Reference") (OtherActor :type "Actor Object Reference") (OtherComp :type "PrimitiveComponent Object Reference") (OtherBodyIndex :type Integer) (bFromSweep :type Boolean) (SweepResult :type "HitResult Structure (by ref)"))
  (bind _returnvalue_x (`KismetMathLibrary.BreakVector` (`SceneComponent.K2_GetComponentLocation` (`self.SM_Wall`))))
  (bind _returnvalue_x_2 (`KismetMathLibrary.BreakVector` (`SceneComponent.K2_GetComponentLocation` (`Actor.RootComponent` (`GameplayStatics.GetPlayerCharacter` 0)))))
  ;[1 0 0] Open Door
  ;[1 1 1] Move SM_Wall ... (animation)
  (bind (_direction _alpha) (`Timeline|Timeline_DoorAnim` :`NewTime` 0.0 :!via `PlayFromStart` :!label _label)
    (:`Update`
      (if (< _returnvalue_x _returnvalue_x_2)
        (`SceneComponent.K2_SetRelativeRotation` (`self.SM_Wall`) (`KismetMathLibrary.RLerp` (struct :`Yaw` 90.0) (struct :`Yaw` 172.0) _alpha true) false false)
        (else
          (`SceneComponent.K2_SetRelativeRotation` (`self.SM_Wall`) (`KismetMathLibrary.RLerp` (struct :`Yaw` 90.0) (struct :`Yaw` 6.88) _alpha true) false false))))))

(event `self.BoxFront.OnComponentEndOverlap`
  (params (OverlappedComponent :type "PrimitiveComponent Object Reference") (OtherActor :type "Actor Object Reference") (OtherComp :type "PrimitiveComponent Object Reference") (OtherBodyIndex :type Integer))
  (goto _label :!via `ReverseFromEnd`))

(event `self.ReceiveTick`
  (params (DeltaSeconds :type "Float (single-precision)")))

(fn `UserConstructionScript`)
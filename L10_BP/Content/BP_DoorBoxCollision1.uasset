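; Door Blueprint that raises a wall mesh while the player character is inside a trigger box and lowers it otherwise.
; Tick polls the box overlap and nudges SMWall along local Z in fixed, frame-rate-dependent steps.
; A LocalOffsetY counter, stepped separately from the mesh offset, limits travel between zero and MAXDOOR.
; An unconnected distance-based scaling test with debug prints remains in the graph and never runs.
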(event `self.Box.OnComponentBeginOverlap`
  (params (OverlappedComponent :type "PrimitiveComponent Object Reference") (OtherActor :type "Actor Object Reference") (OtherComp :type "PrimitiveComponent Object Reference") (OtherBodyIndex :type Integer) (bFromSweep :type Boolean) (SweepResult :type "HitResult Structure (by ref)"))
  ;[1 1 1] Player near
)

(event `self.ReceiveTick`
  (params (DeltaSeconds :type "Float (single-precision)"))
  (bind _returnvalue (+ (`self.local_offset_y`) -0.2))
  (bind _returnvalue_2 (+ (`self.local_offset_y`) 0.2))
  (if (`PrimitiveComponent.IsOverlappingActor` (`self.Box`) (`GameplayStatics.GetPlayerCharacter` 0))
    (if (not (> _returnvalue_2 (`self.MAX_DOOR`)))
      (set `self.local_offset_y` _returnvalue_2)
      (`SceneComponent.K2_AddLocalOffset` (`self.SM_Wall`) (0.0 0.0 1.0) false false))
    (elif (not (<= _returnvalue 0.0))
      (set `self.local_offset_y` _returnvalue)
      (`SceneComponent.K2_AddLocalOffset` (`self.SM_Wall`) (0.0 0.0 -1.0) false false))))

(fn `UserConstructionScript`)
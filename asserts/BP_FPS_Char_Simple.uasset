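; BP_FPS_Char_Simple is a minimal first-person character with keyboard movement and mouse look.
; Tick polls the W, A, S and D keys directly on player controller 0 rather than using mapped movement inputs, turning them into forward and right movement along the actor's axes.
; MouseX and MouseY axis events drive controller yaw and pitch, with an optional InvertMouseY flip.
; BeginPlay sets focus to the game viewport.
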(event `self.ReceiveBeginPlay`
  (`WidgetBlueprintLibrary.SetFocusToGameViewport`))

(event `self.ReceiveTick`
  (params (DeltaSeconds :type "Float (single-precision)"))
  (bind _returnvalue (`GameplayStatics.GetPlayerController` 0))
  (bind _returnvalue_2 (`GameplayStatics.GetPlayerController` 0))
  (`self.AddMovementInput` (`self.GetActorForwardVector`) (+ (* (`KismetMathLibrary.Conv_BoolToDouble` (`PlayerController.IsInputKeyDown` _returnvalue_2 "S")) -1.0) (`KismetMathLibrary.Conv_BoolToDouble` (`PlayerController.IsInputKeyDown` _returnvalue_2 "W"))))
  (`self.AddMovementInput` (`self.GetActorRightVector`) (+ (* (`KismetMathLibrary.Conv_BoolToDouble` (`PlayerController.IsInputKeyDown` _returnvalue "A")) -1.0) (`KismetMathLibrary.Conv_BoolToDouble` (`PlayerController.IsInputKeyDown` _returnvalue "D")))))

(event `InputAxisKey|MouseX`
  (params (AxisValue :type "Float (single-precision)"))
  (`self.AddControllerYawInput` AxisValue))

(event `InputAxisKey|MouseY`
  (params (AxisValue :type "Float (single-precision)"))
  (`self.AddControllerPitchInput` (* AxisValue (select `bool` (`self.InvertMouseY`) :`false` 1.0 :`true` -1.0 :!type "Float (single-precision)"))))

(fn `UserConstructionScript`)